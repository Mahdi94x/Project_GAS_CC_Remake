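; Base death ability for Crash Course characters, handling death and respawn.
; On activation it plays the death montage and applies GE_Death to the owner.
; When the montage completes, is interrupted or is cancelled, it removes the Status.Dead effect and caches the avatar character.
; Only the authority resets attributes and moves the character to a GameMode player start, then HandleRespawn runs and the ability ends.
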(event `self.K2_ActivateAbility`
  (`AbilityTask_PlayMontageAndWait.CreatePlayMontageAndWaitProxy` "None" (`self.DeathMontage`)
    (:`then`
      (`self.GrantingStatusDeathTag`))
    (:`OnCompleted`
      (`self.RespawnCharacter` :!label _label))
    (:`OnInterrupted`
      (goto _label))
    (:`OnCancelled`
      (goto _label))))

(event `RespawnCharacter`
  (`|ExecutionSequence`
    (:`then_0`
      (`self.BP_RemoveGameplayEffectFromOwnerWithGrantedTags` (struct :`GameplayTags` (struct :`(TagName` "CCTags.Status.Dead"))) 1))
    (:`then_1`
      ;[0.04054 0.05552 0.15 0.5] Caching CC Base Character
      (bind _ascc_base_character (cast `CC_BaseCharacter` (`self.GetAvatarActorFromActorInfo`)))
      (set `self.CC Base Character` _ascc_base_character))
    (:`then_2`
      ;[0.15 0.1306 0.001164 0.5] Only Server
      (`self.K2_HasAuthority`
        (:`True`
          (`|ExecutionSequence`
            (:`then_0`
              ;;[0.04054 0.05552 0.15 0.5] Resetting Attributes
              (bind _cc_base_character (`self.CC Base Character`)
                (:`then`
                  (`CC_BaseCharacter.ResetAttributes` _cc_base_character))
                (:`else`)))
            (:`then_1`
              ;;[0.04054 0.05552 0.15 0.5] Teleporting the Character
              (bind _cc_base_character_2 (`self.CC Base Character`)
                (:`then`
                  (`Actor.K2_SetActorLocation` (`self.CC Base Character`) (`Actor.K2_GetActorLocation` (`GameModeBase.K2_FindPlayerStart` (`GameplayStatics.GetGameMode`) (`Pawn.GetController` _cc_base_character_2) "")) false false))
                (:`else`)))))))
    (:`then_3`
      (bind _cc_base_character_3 (`self.CC Base Character`)
        (:`then`
          (`CC_BaseCharacter.HandleRespawn` _cc_base_character_3))
        (:`else`)))
    (:`then_4`
      (`self.K2_EndAbility`))))

(fn `GrantingStatusDeathTag`
  (bind _returnvalue (`self.GetAbilitySystemComponentFromActorInfo`))
  (`AbilitySystemComponent.BP_ApplyGameplayEffectSpecToSelf` _returnvalue (`AbilitySystemComponent.MakeOutgoingSpec` :`self` _returnvalue :`GameplayEffectClass` "/Game/CrashCourse/GameplayAbilitySystem/Effects/GE_Death.GE_Death_C" :`Level` 1.0)))