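; Base Gameplay Ability that plays directional hit reactions in response to the enemy HitReact gameplay event.
; On activation it waits for that event, then either ends and sends EndAttack to the avatar if it is dead, or computes the hit direction from the instigator.
; The direction name selects the HitReactMontage section to jump to, and the ability ends when the montage finishes or is interrupted.
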(event `self.K2_ActivateAbility`
  (bind (_asynctaskproxy _payload) (`AbilityTask_WaitGameplayEvent.WaitGameplayEvent` (struct :`TagName` "CCTags.Events.Enemy.HitReact") null)
    (:`EventReceived`
      (if (`GameplayTagAssetInterface.HasMatchingGameplayTag` (`self.GetAbilitySystemComponentFromActorInfo`) (struct :`TagName` "CCTags.Status.Dead"))
        (`self.K2_EndAbility`)
        (`AbilitySystemBlueprintLibrary.SendGameplayEventToActor` (`self.GetAvatarActorFromActorInfo`) (struct :`TagName` "CCTags.Events.Enemy.EndAttack"))
        (else
          (`self.PrintDebugEventReceived` _payload)
          (`self.CacheHitDirectionVectors` (`.Instigator` (break `GameplayEventData` _payload)))
          (`|ExecutionSequence`
            (:`then_0`
              ;[0.15 0.0286 0.1352 0.5] Cache HitDirectionName
              (set `self.HitDirectionName` (`CC_BlueprintLibrary.GetHitDirectionName` (`CC_BlueprintLibrary.GetHitDirection` (`self.AvatarForward`) (`self.ToInstigator`))))
              ;[0.15 0.02114 0.009399 0.5] Debug For Hit Direction
              (`self.bDrawDebugs`
                (:`then`
                  (`KismetSystemLibrary.PrintString` (`KismetStringLibrary.Conv_NameToString` (`self.HitDirectionName`)) true true (struct :`G` 0.66 :`B` 1.0 :`A` 1.0) 5.0))
                (:`else`)))
            (:`then_1`
              ;[0.15 0.1461 0 0.5] Play Montage Hit React Section
              (`AbilityTask_PlayMontageAndWait.CreatePlayMontageAndWaitProxy` "None" (`self.HitReact Montage`)
                (:`then`
                  (`self.MontageJumpToSection` (`self.HitDirectionName`)))
                (:`OnCompleted`
                  (`self.K2_EndAbility` :!label _label))
                (:`OnBlendOut`
                  (goto _label))
                (:`OnInterrupted`
                  (goto _label))
                (:`OnCancelled`
                  (goto _label))))))))))

(fn `PrintDebugEventReceived`
  (params (GameplayEventData :type "GameplayEventData Structure (by ref)"))
  (bind (_eventtag _instigator) (break `GameplayEventData` GameplayEventData))
  (`self.bDrawDebugs`
    (:`then`
      (`KismetSystemLibrary.PrintString` (`KismetStringLibrary.Concat_StrStr` "GA_CC_HitReact Received Event from ----> " (`KismetSystemLibrary.GetDisplayName` _instigator) " ---> Tag Received is ----> " (`BlueprintGameplayTagLibrary.GetDebugStringFromGameplayTag` _eventtag)) true true (struct :`G` 0.66 :`B` 1.0 :`A` 1.0) 5.0))
    (:`else`)))