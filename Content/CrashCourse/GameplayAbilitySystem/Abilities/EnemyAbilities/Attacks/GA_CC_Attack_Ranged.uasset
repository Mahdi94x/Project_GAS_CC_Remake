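; Gameplay ability for an enemy ranged attack in CrashCourse.
; On activation it plays the attack montage and, on the authority, immediately spawns a projectile owned by the avatar and sends it the EndAttack gameplay event.
; FlatProjectileZ builds the spawn transform from the front muzzle socket, flattening its forward vector so shots launch horizontally.
; The ability ends when the montage completes, is interrupted or is cancelled.
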(event `self.K2_ActivateAbility`
  (`AbilityTask_PlayMontageAndWait.CreatePlayMontageAndWaitProxy` "None" "/Game/CrashCourse/Characters/EnemyCharacter/Ranged/Animation/AM_EnemyAttack_Ranged.AM_EnemyAttack_Ranged" 1.0 "None" false
    (:`then`
      (`self.K2_HasAuthority`
        (:`True`
          (`|SpawnActorFromClass` "/Game/CrashCourse/GameObjects/BP_CC_Projectile.BP_CC_Projectile_C" (`self.FlatProjectileZ`) "Undefined" "MultiplyWithRoot" (`self.GetAvatarActorFromActorInfo`) 25.0 null)
          (`AbilitySystemBlueprintLibrary.SendGameplayEventToActor` (`self.GetAvatarActorFromActorInfo`) (struct :`TagName` "CCTags.Events.Enemy.EndAttack")))))
    (:`OnCompleted`
      (`self.K2_EndAbility` :!label _label))
    (:`OnInterrupted`
      (goto _label))
    (:`OnCancelled`
      (goto _label))))

(fn `FlatProjectileZ`
  (returns (ReturnValue :type "Transform Structure"))
  (bind (_returnvalue_location _returnvalue_rotation _returnvalue_scale) (`KismetMathLibrary.BreakTransform` (`SceneComponent.GetSocketTransform` (`self.GetOwningComponentFromActorInfo`) "Muzzle_Front" "RTS_World")))
  (bind (_returnvalue_x _returnvalue_y) (`KismetMathLibrary.BreakVector` (`KismetMathLibrary.GetForwardVector` _returnvalue_rotation)))
  (return (`KismetMathLibrary.MakeTransform` _returnvalue_location (`KismetMathLibrary.MakeRotFromX` (`KismetMathLibrary.MakeVector` _returnvalue_x _returnvalue_y)) _returnvalue_scale)))