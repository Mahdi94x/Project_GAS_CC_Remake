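; Enemy melee attack gameplay ability that plays a random attack montage and damages the player on a trace hit.
; If the avatar is tagged dead it ends immediately; otherwise it runs the montage alongside a one-shot wait for the MeleeTraceHit event.
; A hit sends fixed SetByCaller melee damage with impact particles to the event's target.
; The ability ends with the montage, and ending sends EndAttack to the avatar.
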(event `self.K2_ActivateAbility`
  (if (`GameplayTagAssetInterface.HasMatchingGameplayTag` (`self.GetAbilitySystemComponentFromActorInfo`) (struct :`TagName` "CCTags.Status.Dead"))
    (`self.K2_EndAbility`)
    (`AbilitySystemBlueprintLibrary.SendGameplayEventToActor` (`self.GetAvatarActorFromActorInfo`) (struct :`TagName` "CCTags.Events.Enemy.EndAttack"))
    (else
      (`|ExecutionSequence`
        (:`then_0`
          ;[0.003411 0.15 0.1471] Play Attack Montage
          (`AbilityTask_PlayMontageAndWait.CreatePlayMontageAndWaitProxy` "None" (`KismetArrayLibrary.Array_Random` (`self.AttackMontages`)) 1.0 "None" false
            (:`OnCompleted`
              _)
            (:`OnBlendOut`
              _)
            (:`OnInterrupted`
              _)
            (:`OnCancelled`
              _))
          (`self.K2_EndAbility`))
        (:`then_1`
          (bind (_asynctaskproxy _payload) (`AbilityTask_WaitGameplayEvent.WaitGameplayEvent` (struct :`TagName` "CCTags.Events.Enemy.MeleeTraceHit") null true)
            (:`EventReceived`
              (`CC_BlueprintLibrary.SendDamageEventToPlayer` (`.Target` (break `GameplayEventData` _payload)) (`self.Melee Damage Effect`) _payload (`BlueprintGameplayTagLibrary.MakeLiteralGameplayTag` (struct :`TagName` "CCTags.SetByCaller.Melee")) 50.0 (`self.ImpactParticles`)))))))))

(event `self.K2_OnEndAbility`
  (params (bWasCancelled :type Boolean))
  (`AbilitySystemBlueprintLibrary.SendGameplayEventToActor` (`self.GetAvatarActorFromActorInfo`) (struct :`TagName` "CCTags.Events.Enemy.EndAttack")))