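; Player primary melee attack ability that alternates between two attack montages on each activation and ends when the montage finishes or is interrupted.
; On activation it applies a block-hit-react effect to the owner, removed again when the ability ends.
; A montage-driven gameplay event triggers a hitbox overlap test, sends hit-react events to those hit and applies level-scaled player damage to each.
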(event `self.K2_ActivateAbility`
  (bind _returnvalue (`self.GetAbilitySystemComponentFromActorInfo`))
  (bind _returnvalue_2 (`self.GetAbilitySystemComponentFromActorInfo`))
  (`|ExecutionSequence`
    (:`then_0`
      ;[0.04054 0.05552 0.15 0.5] Apply Blck Hit React GE
      (`AbilitySystemComponent.BP_ApplyGameplayEffectSpecToSelf` _returnvalue (`AbilitySystemComponent.MakeOutgoingSpec` :`self` _returnvalue :`GameplayEffectClass` "/Game/CrashCourse/GameplayAbilitySystem/Effects/Player/GE_BlockHitReact.GE_BlockHitReact_C" :`Level` 1.0)))
    (:`then_1`
      ;[0.02221 0.04074 0.15 0.5] Play Primary Attack Montage
      (`/Engine/EditorBlueprintResources/StandardMacros.FlipFlop`
        (:`A`
          (`AbilityTask_PlayMontageAndWait.CreatePlayMontageAndWaitProxy` "None" "/Game/CrashCourse/Characters/PlayerCharacter/Animations/Montages/CC_Primary_A_Montage.CC_Primary_A_Montage"
            (:`OnCompleted`
              _)
            (:`OnBlendOut`
              _)
            (:`OnInterrupted`
              _)
            (:`OnCancelled`
              _))
          (`self.K2_EndAbility`))
        (:`B`
          (`AbilityTask_PlayMontageAndWait.CreatePlayMontageAndWaitProxy` "None" "/Game/CrashCourse/Characters/PlayerCharacter/Animations/Montages/CC_Primary_B_Montage.CC_Primary_B_Montage"
            (:`OnCompleted`
              _)
            (:`OnBlendOut`
              _)
            (:`OnInterrupted`
              _)
            (:`OnCancelled`
              _))
          (`self.K2_EndAbility`))))
    (:`then_2`
      ;[0.04054 0.05552 0.15 0.5] Perform Overlap Test and Send HitReact Event
      (`AbilityTask_WaitGameplayEvent.WaitGameplayEvent` (struct :`TagName` "CCTags.Events.Player.Primary") null
        (:`EventReceived`
          (bind _returnvalue_3 (`CC_BlueprintLibrary.HitBoxOverlapTest` (`self.GetAvatarActorFromActorInfo`) (`self.HitBoxRadius`) (`self.HitBoxForwardOffset`) (`self.HitBoxElevationOffset`) (`self.bDrawDebugs`)))
          (`self.SendHitReactEventsToActor` _returnvalue_3)
          (for _array_element _returnvalue_3
            (`AbilitySystemComponent.BP_ApplyGameplayEffectSpecToTarget` _returnvalue_2 (`AbilitySystemComponent.MakeOutgoingSpec` :`self` _returnvalue_2 :`GameplayEffectClass` "/Game/CrashCourse/GameplayAbilitySystem/Effects/Player/GE_PlayerDamage.GE_PlayerDamage_C" :`Level` (`KismetMathLibrary.Conv_IntToDouble` (`self.GetAbilityLevel`))) (`AbilitySystemBlueprintLibrary.GetAbilitySystemComponent` _array_element))))))))

(event `self.K2_OnEndAbility`
  (params (bWasCancelled :type Boolean))
  (`self.BP_RemoveGameplayEffectFromOwnerWithGrantedTags` (struct :`GameplayTags` (struct :`(TagName` "CCTags.CCAbilities.BlockHitReact"))) 1))