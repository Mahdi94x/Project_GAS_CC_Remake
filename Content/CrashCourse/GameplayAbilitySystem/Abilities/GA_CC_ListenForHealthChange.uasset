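; GA_CC_ListenForHealthChange is a gameplay ability that watches its owner's health and triggers death when it reaches zero or below.
; On activation it starts an async attribute-change listener on the owner's Ability System Component and stores the task.
; Each change optionally prints debug text and, at zero or less, activates abilities by the Death tag, allowing remote activation.
; When the ability ends, it ends the stored listener task.
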(event `self.K2_ActivateAbility`
  (bind (_asynctaskproxy _attribute _oldvalue _newvalue) (`CC_AttributeChangeTask.ListenForAttributeChange` (`self.GetAbilitySystemComponentFromActorInfo`) (struct :`AttributeName` "Health" :`Attribute` "/Script/Project_GAS_CC.CC_AttributeSet:Health" :`AttributeOwner` "/Script/CoreUObject.Class'/Script/Project_GAS_CC.CC_AttributeSet'"))
    (:`then`
      (set `self.AttributeChangeTask` _asynctaskproxy))
    (:`OnAttributeChanged`
      (`self.DebugPrintNewHealthValue` _newvalue)
      (if (<= _newvalue 0.0)
        (`AbilitySystemComponent.TryActivateAbilitiesByTag` (`self.GetAbilitySystemComponentFromActorInfo`) (`BlueprintGameplayTagLibrary.MakeLiteralGameplayTagContainer` (struct :`GameplayTags` (struct :`(TagName` "CCTags.CCAbilities.Death")))) true)))))

(event `self.K2_OnEndAbility`
  (params (bWasCancelled :type Boolean))
  (bind _attributechangetask (`self.AttributeChangeTask`)
    (:`then`
      (`CC_AttributeChangeTask.EndTask` _attributechangetask))
    (:`else`)))

(fn `DebugPrintNewHealthValue`
  (params (NewAttributeValue :type "Float (double-precision)"))
  (`self.bDrawDebugs`
    (:`then`
      (`KismetSystemLibrary.PrintString` (`KismetStringLibrary.Concat_StrStr` "GA_CC_ListenForHealthChange Activated for   " (`KismetSystemLibrary.GetDisplayName` (`self.GetAvatarActorFromActorInfo`)) " New Health Value is:" (`KismetStringLibrary.Conv_DoubleToString` NewAttributeValue)) true true (struct :`R` 1.0 :`B` 0.004563 :`A` 1.0) 3.0))
    (:`else`)))